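; BP_SnakeTail is a snake tail segment that follows the segment ahead and takes its material from its color.
; It binds to the next segment's step-start event to move, stepping after a fifth of StepTime.
; Relinking to a new next segment rebinds that event and skips one step.
; TakeEndTailColor recurses backward to the last segment, destroys it, and returns its color.
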(event Custom|ce_MoveToNextSegment
  (if (Variables|Default|GetSkipStep)
    (Variables|Default|SetSkipStep false)
    (else
      (Utilities|FlowControl|Delay (* (Variables|Default|GetStepTime) 0.2))
      (CallFunction|CeDoStep))))

(event EventBeginPlay
  (|CallParentFunction)
  (Rendering|Material|SetMaterial (Variables|Default|GetSegment) 0 (CallFunction|GetMaterialbyColor (Variables|Default|GetSegmentColor)))
  (EventDispatchers|BindEventtoEDStartStep (Variables|Default|GetNextSegmentRef) (EventDispatchers|CreateEvent :!event Custom|ce_MoveToNextSegment)))

(event EventSetNextSegment
  (params (NewSegment :type BP%20Base%20Snake%20Segment%20Object%20Reference))
  ;[1 1 1] Unbind old segment, skip 1 step and bind to new next segment
  (EventDispatchers|UnbindEventfromEDStartStep (Variables|Default|GetNextSegmentRef) (EventDispatchers|CreateEvent :!event Custom|ce_MoveToNextSegment))
  (Variables|Default|SetSkipStep true)
  (bind _output_get (Variables|Default|SetNextSegmentRef NewSegment))
  (EventDispatchers|BindEventtoEDStartStep _output_get (EventDispatchers|CreateEvent :!event Custom|ce_MoveToNextSegment)))

(fn ConstructionScript
  (|CallParentFunction))

(fn TakeEndTailColor
  (bind _backsegmentref (Variables|Default|GetBackSegmentRef))
  (Utilities|IsValid _backsegmentref
    (:Is%20Valid
      (bind _color (Default|TakeEndTailColor _backsegmentref))
      (return _color))
    (:Is%20Not%20Valid
      (CallFunction|CeDestroySegment)
      (return (Variables|Default|GetSegmentColor)))))