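; BP_GameObject is a game object that occupies a floor cell and awards score when destroyed.
; On BeginPlay it applies a random colour material to InteractObject, stores the matching segment colour, and marks its cell occupied through the game mode.
; Its destroy event sets the cell status from ClearPlace, reports its class and score to the game mode, then destroys the actor.
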(event Custom|ce_EventOnSpawn
  (Class|BPIGameMode|SetStatusCellonFloor(Message) (Game|GetGameMode) (Transformation|GetActorLocation) false))

(event Custom|ce_OnDestroy
  (params (ClearPlace :type Boolean))
  (bind _returnvalue (Game|GetGameMode))
  (Class|BPIGameMode|SetStatusCellonFloor(Message) _returnvalue (Transformation|GetActorLocation) ClearPlace)
  (Class|BPIGameMode|GameObjectDestroyed(Message) _returnvalue (Utilities|GetClass self))
  (CallFunction|AddScore)
  (Actor|DestroyActor))

(event EventBeginPlay
  (|CallParentFunction)
  (CallFunction|SetRandomMaterial)
  (CallFunction|CeEventonSpawn))

(fn ConstructionScript)

(fn AddScore
  (Class|BPIGameMode|AddScore(Message) (Game|GetGameMode) (Variables|Default|GetScore))
  (return))

(fn SetRandomMaterial
  (bind (_material _colorindex) (CallFunction|GetRandomMaterialbyColor))
  (Rendering|Material|SetMaterial (Variables|Default|GetInteractObject) 0 _material)
  (Variables|Default|SetObjectColor (Utilities|Enum|ByteToEnumE_SegmentColors (Math|Conversions|ToByte(Integer) _colorindex)))
  (return))