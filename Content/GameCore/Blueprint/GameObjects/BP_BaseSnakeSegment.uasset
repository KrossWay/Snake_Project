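; Base actor for one snake segment, moving one grid cell (a meter) per step and reporting cell occupancy to the game mode.
; Segments form a linked chain: the head follows non-reversing input, while the others take the next segment's old position.
; A per-frame looping timer lerps each step, then snaps to grid.
; Stopping and delayed shrink-and-destroy cascade toward the tail, whose last segment reports player death.
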(event Custom|ce_DoStep
  ;[1 1 1] Do one step. Step duration == StepTime
  (CallFunction|TakeInputDirection)
  (CallFunction|SetMovePosition)
  (if (not (Variables|Status|GetIsDie))
    (Variables|MoveParameters|SetStepCounter 0.0)
    (Default|CallEDStartStep)
    (CallFunction|UpdateCellLocationinArea)
    (bind _returnvalue (Utilities|Time|SetTimerbyEvent (EventDispatchers|CreateEvent :!event StepMove) (Utilities|Time|GetWorldDeltaSeconds) true))
    (Variables|MoveParameters|SetDoStepTimer _returnvalue)))

(event Custom|ce_StopAllMoving
  (bind _backsegmentref (Variables|Object|GetBackSegmentRef))
  ;[1 1 1] Stop moving, clear all timers
  (Utilities|Time|ClearandInvalidateTimerbyHandle (Variables|MoveParameters|GetDoStepTimer))
  (Variables|Status|SetIsDie true)
  (Utilities|IsValid _backsegmentref
    (:Is%20Valid
      (CallFunction|CeStopAllMoving _backsegmentref))))

(event Custom|ce_DestroyBackWithDelay
  (params (Delay :type Float%20%28single-precision%29))
  (bind _backsegmentref (Variables|Object|GetBackSegmentRef))
  ;[1 1 1] Begin destroy self segment and call destroy back segment with delay
  (CallFunction|CeCollapseSegment)
  (Utilities|FlowControl|Delay Delay)
  (Utilities|IsValid _backsegmentref
    (:Is%20Valid
      (CallFunction|CeDestroyBackwithDelay _backsegmentref Delay))
    (:Is%20Not%20Valid
      (CallFunction|SnakeIsDead))))

(event Custom|ce_DestroySegment
  ;[1 1 1] Event on Actor Destroyed
  (Class|BPIGameMode|SetStatusCellonFloor(Message) (Game|GetGameMode) (Transformation|GetActorLocation) true)
  (Actor|DestroyActor))

(event Custom|ce_CollapseSegment
  ;[1 1 1] Decrease scale, then destroy actor
  (Variables|MoveParameters|SetInitialScale (Transformation|GetWorldScale (Variables|Default|GetSegment)))
  (Default|ClearBackSegment (Variables|Object|GetNextSegmentRef))
  (bind _alpha (Timeline|Timeline_0 Play)
    (:Update
      (Transformation|SetWorldScale3D (Variables|Default|GetSegment) (Math|Vector|Lerp(Vector) (Variables|MoveParameters|GetInitialScale) "0, 0, 0" _alpha)))
    (:Finished
      (CallFunction|CeDestroySegment))))

(event EventDestroyChainSegments
  (params (Delay :type Float%20%28single-precision%29))
  (CallFunction|CeDestroyBackwithDelay Delay))

(event EventClearBackSegment
  (Variables|Object|SetBackSegmentRef 0))

(event EventBeginPlay
  (CallFunction|InitializePositionandDirection)
  (Class|BPIGameMode|SetStatusCellonFloor(Message) (Game|GetGameMode) (Transformation|GetActorLocation) false))

(fn ConstructionScript)

(fn StepMove
  (Variables|MoveParameters|SetStepCounter (+ (Variables|MoveParameters|GetStepCounter) (Utilities|Time|GetWorldDeltaSeconds)))
  (Transformation|SetActorLocation (Math|Vector|Lerp(Vector) (Variables|MoveParameters|GetOldPosition) (Variables|MoveParameters|GetNewPosition) (Math|Float|MapRangeClamped (+ (Variables|MoveParameters|GetStepCounter) (Utilities|Time|GetWorldDeltaSeconds)) 0.0 (Variables|MoveParameters|GetStepTime) 0.0 1.0)) true false)
  (if (>= (Variables|MoveParameters|GetStepCounter) 1.0)
    (Transformation|SetActorLocation (Utilities|RoundVectortoMeter (Variables|MoveParameters|GetNewPosition)) true false)
    (Utilities|Time|ClearandInvalidateTimerbyHandle (Variables|MoveParameters|GetDoStepTimer))))

(fn SwitchDirection
  (params (InputValue :type Float%20%28single-precision%29) (IsRightInput :type Boolean))
  (if (> InputValue 0.0)
    (Variables|MoveParameters|SetInputDirection (select IsRightInput "0.000000,90.000000, 0" "0, 0, 0"))
    (else
      (Variables|MoveParameters|SetInputDirection (select IsRightInput "0.000000,-90.000000, 0" "0.000000,-180.000000, 0")))))

(fn TakeInputDirection
  (Utilities|IsValid (Variables|Object|GetNextSegmentRef)
    (:Is%20Not%20Valid
      ;[1 1 1] If valid this is head
      (if (CallFunction|DirectionIsNotOpposite)
        (Variables|MoveParameters|SetCurrentDirection (Variables|MoveParameters|GetInputDirection))
        (return)))))

(fn SetMovePosition
  (bind _returnvalue (Transformation|GetActorLocation))
  (Variables|MoveParameters|SetOldPosition _returnvalue)
  (Utilities|IsValid (Variables|Object|GetNextSegmentRef)
    (:Is%20Valid
      ;[1 1 1] If valid this is tail, take next segment position
      (Variables|MoveParameters|SetNewPosition (Variables|BP_BaseSnakeSegment_C|GetOldPosition (Variables|Object|GetNextSegmentRef)))
      (return))
    (:Is%20Not%20Valid
      ;[1 1 1] If is not valid this is head, take input direction
      (Variables|MoveParameters|SetNewPosition (+ _returnvalue (* (Math|Vector|GetForwardVector (Variables|MoveParameters|GetCurrentDirection)) (CallFunction|GetOneMeterConst))))
      (return))))

(fn DirectionIsNotOpposite
  (return (Utilities|Enum|NotEqual(Enum) (Variables|MoveParameters|GetInputDirection) (Math|Rotator|CombineRotators (Variables|MoveParameters|GetCurrentDirection) "0,180.000000, 0") 0.1)))

(fn InitializePositionandDirection
  (Variables|MoveParameters|SetInputDirection (Math|Conversions|RotationFromXVector (Transformation|GetActorForwardVector)))
  ;[1 1 1] info for back segment
  (Variables|MoveParameters|SetOldPosition (Transformation|GetActorLocation))
  (return))

(fn UpdateCellLocationinArea
  (Utilities|IsValid (Variables|Object|GetNextSegmentRef)
    (:Is%20Valid
      _)
    (:Is%20Not%20Valid
      (Class|BPIGameMode|SetStatusCellonFloor(Message) (Game|GetGameMode) (Variables|MoveParameters|GetNewPosition) false)))
  (Utilities|IsValid (Variables|Object|GetBackSegmentRef)
    (:Is%20Valid
      _)
    (:Is%20Not%20Valid
      (Class|BPIGameMode|SetStatusCellonFloor(Message) (Game|GetGameMode) (Variables|MoveParameters|GetOldPosition) true)))
  (return))

(fn SnakeIsDead
  (Class|BPIGameMode|PlayerIsDead(Message) (Game|GetGameMode)))

(fn GetNextSegment
  (return (Variables|Object|GetNextSegmentRef)))

(fn TakeEndTailColor
  ;[1 1 1] For child
  (return "NewEnumerator0"))