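; Player-controlled snake head that steps on a looping timer, steers from axis input and spawns a linked chain of colored BP_SnakeTail segments.
; An eaten ball inserts a matching segment behind the head next step, while firing takes the end tail's color for a projectile.
; Self-overlap stops movement and destroys chain segments; hits kill the snake.
; It also reports grid points around its old, new and predicted positions.
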(event OnComponentBeginOverlap(Sphere)
  (params (OverlappedComponent :type Primitive%20Component%20Object%20Reference) (OtherActor :type Actor%20Object%20Reference) (OtherComp :type Primitive%20Component%20Object%20Reference) (OtherBodyIndex :type Integer) (bFromSweep :type Boolean) (SweepResult :type Hit%20Result%20Structure%20%28by%20ref%29))
  ;[1 1 1] Overlap Event with self tail
  (if (Utilities|DoesObjectImplementInterface OtherActor "/Game/GameCore/Blueprint/Interfaces/BPI_Snake.BPI_Snake_C")
    ;;[1 1 1] Overlap segment is != head back segment
    (bind _nextsegment (Class|BPISnake|GetNextSegment(Message) OtherActor))
    (if (!= _nextsegment self)
      (CallFunction|CeStopAllMoving)
      (Class|BPISnake|DestroyChainSegments(Message) OtherActor 0.3))))

(event Custom|ce_StartGame
  ;[1 1 1] Start Game Event
  (bind _returnvalue (Utilities|Time|SetTimerbyEvent (EventDispatchers|CreateEvent :!event MoveForward) (* (Variables|Default|GetStepTime) 2.0) true))
  (Variables|Timers|SetMoveForwardTimer _returnvalue))

(event EventBeginPlay
  ;[1 1 1] BeginPlay
  (|CallParentFunction)
  (Initialize|InitializeSnakeLength))

(event EventEatBall
  (params (Ball :type BP%20Eat%20Ball%20Object%20Reference))
  ;[1 1 1] If set, insert segment on next step
  (Variables|GameObjects|SetBall Ball))

(event Collision|EventHit
  (params (MyComp :type Primitive%20Component%20Object%20Reference) (Other :type Actor%20Object%20Reference) (OtherComp :type Primitive%20Component%20Object%20Reference) (bSelfMoved :type Boolean) (HitLocation :type Vector :default "0, 0, 0") (HitNormal :type Vector :default "0, 0, 0") (NormalImpulse :type Vector :default "0, 0, 0") (Hit :type Hit%20Result%20Structure%20%28by%20ref%29))
  ;[1 1 1] If Hit to static meshes
  (CallFunction|CeStopAllMoving)
  (CallFunction|SnakeIsDead))

(event EventCeStopAllMoving
  ;[1 1 1] Add clear timer of this class
  (|CallParentFunction)
  (Utilities|Time|ClearandInvalidateTimerbyHandle (Variables|Timers|GetMoveForwardTimer)))

(event EventInputFire
  ;[1 1 1] Player Controller inputs
  (System|TryFireSegment))

(event EventInputMoveUp
  (params (AxisValue :type Float%20%28single-precision%29))
  ;[1 1 1] Player Controller inputs
  (CallFunction|SwitchDirection AxisValue false))

(event EventInputMoveRight
  (params (AxisValue :type Float%20%28single-precision%29))
  ;[1 1 1] Player Controller inputs
  (CallFunction|SwitchDirection AxisValue true))

(event EventBeginMoving
  ;[1 1 1] Event on Game Begin
  (CallFunction|CeStartGame))

(event EventStopGame
  ;[1 1 1] Event on Game Stop
  (if (not (Variables|Default|GetIsDie))
    (CallFunction|CeStopAllMoving)))

(fn ConstructionScript
  (|CallParentFunction))

(fn InitializeSnakeLength
  (Class|BPIGameMode|SetStatusCellonFloor(Message) (Game|GetGameMode) (Transformation|GetActorLocation) false)
  (for _index (range 1 (Variables|Settings|GetSnakeLength))
    (bind _output_get (LocalVariables|SetL_Index _index))
    (bind _colorindex (CallFunction|GetRandomMaterialbyColor))
    (bind _returnvalue (Game|SpawnActorfromClass "/Game/GameCore/Blueprint/GameObjects/BP_SnakeTail.BP_SnakeTail_C" (Math|Transform|MakeTransform (Initialize|NextSpawnSegment _output_get) "0, 0, 0" "1,1,1") "AlwaysSpawn" 0 (Utilities|Enum|ByteToEnumE_SegmentColors (Math|Conversions|ToByte(Integer) _colorindex)) (select (== (LocalVariables|GetL_Index) 1) self (LocalVariables|GetL_NextSegnemt)) 0))
    (if (== (LocalVariables|GetL_Index) 1)
      ;[1 1 1] build a chain of connections
      (bind _output_get_2 (LocalVariables|SetL_NextSegnemt _returnvalue))
      ;;[1 1 1] for self class
      (Variables|Default|SetBackSegmentRef _output_get_2)
      (else
        (Variables|/Game/GameCore/Blueprint/GameObjects/BP_BaseSnakeSegment.BP_BaseSnakeSegment_C|SetBackSegmentRef (LocalVariables|GetL_NextSegnemt) _returnvalue)
        (LocalVariables|SetL_NextSegnemt _returnvalue)))))

(fn NextSpawnSegment
  (params (Index :type Integer))
  (bind _returnvalue (Transformation|GetActorLocation))
  (return (Math|Vector|MakeVector (- (.x _returnvalue) (* Index (Variables|Default|GetOneMeter))) (.y _returnvalue) (.z _returnvalue))))

(fn InsertSegment
  (params (Color :type E_SegmentColors%20Enum :default "NewEnumerator0"))
  (bind _returnvalue (Game|SpawnActorfromClass "/Game/GameCore/Blueprint/GameObjects/BP_SnakeTail.BP_SnakeTail_C" (Math|Transform|MakeTransform (Transformation|GetActorLocation) "0, 0, 0" "1,1,1") "AlwaysSpawn" 0 Color self 0))
  (LocalVariables|SetL_NewSegment _returnvalue)
  (Utilities|IsValid (Variables|Default|GetBackSegmentRef)
    (:Is%20Valid
      (Variables|/Game/GameCore/Blueprint/GameObjects/BP_BaseSnakeSegment.BP_BaseSnakeSegment_C|SetBackSegmentRef (LocalVariables|GetL_NewSegment) (Variables|Default|GetBackSegmentRef))
      (Default|SetNextSegment (Variables|Default|GetBackSegmentRef) (LocalVariables|GetL_NewSegment))
      (Variables|Default|SetBackSegmentRef (LocalVariables|GetL_NewSegment)))
    (:Is%20Not%20Valid
      (Default|SetNextSegment (LocalVariables|GetL_NewSegment) self)
      (Variables|Default|SetBackSegmentRef (LocalVariables|GetL_NewSegment)))))

(fn AddNewSegment
  (System|InsertSegment (Variables|/Game/GameCore/Blueprint/GameObjects/BP_GameObject.BP_GameObject_C|GetObjectColor (Variables|GameObjects|GetBall)))
  (Default|CeEat (Variables|GameObjects|GetBall))
  (Variables|GameObjects|SetBall 0)
  (return))

(fn TryFireSegment
  (bind _backsegmentref (Variables|Default|GetBackSegmentRef))
  (if (not (Variables|Default|GetIsDie))
    ;[1 1 1] Recursion
    (Utilities|IsValid _backsegmentref
      (:Is%20Valid
        (bind _color (Default|TakeEndTailColor _backsegmentref))
        (Game|SpawnActorfromClass "/Game/GameCore/Blueprint/GameObjects/BP_Projectile.BP_Projectile_C" (Math|Transform|MakeTransform (Transformation|GetActorLocation) (Variables|Default|GetCurrentDirection) "1,1,1") "Undefined" 0 _color 0)
        (return))
      (:Is%20Not%20Valid
        (return)))))

(fn MoveForward
  (Utilities|IsValid (Variables|GameObjects|GetBall)
    (:Is%20Valid
      (System|AddNewSegment))
    (:Is%20Not%20Valid
      _))
  (CallFunction|CeDoStep)
  (return))

(fn GetPointsAroundHead
  (bind _centerpoints (Location|ConstructCenterPointsArray))
  (for _array_element _centerpoints
    (bind _rightpoints (Location|GetRightPointsAroundCenter _array_element))
    (Utilities|Array|AppendArray (LocalVariables|GetL_Points) _rightpoints))
  (return (LocalVariables|GetL_Points)))

(fn GetRightPointsAroundCenter
  (params (CenterPoint :type Vector))
  (Utilities|Array|AddUnique (LocalVariables|GetL_Points) CenterPoint)
  (Utilities|Array|AddUnique (LocalVariables|GetL_Points) (Utilities|GetRightMeterPoint CenterPoint false))
  (Utilities|Array|AddUnique (LocalVariables|GetL_Points) (Utilities|GetRightMeterPoint CenterPoint true))
  (return (LocalVariables|GetL_Points)))

(fn ConstructCenterPointsArray
  (bind _newposition (Variables|Default|GetNewPosition))
  ;[1 1 1] We need first point old position, second point new position, third point position
  ; envisioned next step
  (return (Utilities|Array|MakeArray (Variables|Default|GetOldPosition) _newposition (+ _newposition (* (Math|Vector|GetForwardVector (Variables|Default|GetCurrentDirection)) (Variables|Default|GetOneMeter))))))

(fn GetPointsAroundPawn
  (bind _points (Location|GetPointsAroundHead))
  (return _points))