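; Level generator actor that builds a resizable checkerboard arena with a block wall border and tracks which cells are empty.
; Floor and walls are instanced meshes built in the construction script on a one-meter grid.
; BeginPlay centers the actor and fills a map of integer cells to empty flags, which ResizeGrid also rebuilds.
; Random empty-point queries first mark points reported by the player controller as occupied.
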(event EventBeginPlay
  (ConstructArena|SetFloortoEqualCenterCoordinate)
  (ConstructArena|GeneratePointsMapList))

(fn ConstructionScript
  (ConstructArena|ConstructFloor)
  (ConstructArena|ConstructBlockWalls))

(fn GetPositionbyIndex
  (params (XIndex :type Integer) (YIndex :type Integer))
  (bind _returnvalue (Transformation|GetActorLocation))
  (return (Math|Vector|MakeVector (+ (* XIndex (CallFunction|GetOneMeterConst)) (.x _returnvalue)) (+ (.y _returnvalue) (* YIndex (CallFunction|GetOneMeterConst))) (.z _returnvalue))))

(fn ConstructFloor
  ;[1 1 1] Create floor chess board
  (Components|InstancedStaticMesh|ClearInstances (Variables|Default|GetInstancedBlackCube))
  (Components|InstancedStaticMesh|ClearInstances (Variables|Default|GetInstanceWhiteCube))
  (for _index (range 0 (- (Variables|Params|GetWidthX) 1))
    (bind _output_get (LocalVariables|SetL_XIndex _index))
    (LocalVariables|SetL_InvertColor (Utilities|IsNotWhole _output_get))
    (for _index_2 (range 0 (- (Variables|Params|GetWidthY) 1))
      (bind _output_get_2 (LocalVariables|SetL_YIndex _index_2))
      (if (Utilities|IsNotWhole _output_get_2)
        (Class|InstancedStaticMeshComponent|AddInstanceWorldSpace (select (LocalVariables|GetL_InvertColor) (Variables|Default|GetInstanceWhiteCube) (Variables|Default|GetInstancedBlackCube)) (Math|Transform|MakeTransform (ConstructArena|GetPositionbyIndex (LocalVariables|GetL_XIndex) (LocalVariables|GetL_YIndex)) "0, 0, 0" "1,1,1"))
        (else
          (Class|InstancedStaticMeshComponent|AddInstanceWorldSpace (select (LocalVariables|GetL_InvertColor) (Variables|Default|GetInstancedBlackCube) (Variables|Default|GetInstanceWhiteCube)) (Math|Transform|MakeTransform (ConstructArena|GetPositionbyIndex (LocalVariables|GetL_XIndex) (LocalVariables|GetL_YIndex)) "0, 0, 0" "1,1,1")))))))

(fn SetFloortoEqualCenterCoordinate
  (bind (_x _y _z) (Math|Vector|BreakVector "0, 0,-50.000000"))
  (Transformation|SetActorLocation (Math|Vector|MakeVector (- _x (* (/ (Variables|Params|GetWidthX) 2) (CallFunction|GetOneMeterConst))) (- _y (* (/ (Variables|Params|GetWidthY) 2) (CallFunction|GetOneMeterConst))) _z) false false)
  (return))

(fn ConstructBlockWalls
  (Components|InstancedStaticMesh|ClearInstances (Variables|Default|GetInstancedBlockWalls))
  ;[1 1 1] Construct Box walls Width X+2 and Y+2 size.
  (LocalVariables|SetL_StartPoint (Utilities|TakeOffsetActorVector))
  ;;[1 1 1] Because numeration loops from zero
  (LocalVariables|SetL_BoxSizeX (+ (Variables|Params|GetWidthX) 1))
  (LocalVariables|SetL_BoxSizeY (+ (Variables|Params|GetWidthY) 1))
  (for _index (range 0 (LocalVariables|GetL_BoxSizeX))
    ;[1 1 1] Create two walls from X coordinate
    (Class|InstancedStaticMeshComponent|AddInstanceWorldSpace (Variables|Default|GetInstancedBlockWalls) (Math|Transform|MakeTransform (Math|Vector|MakeVector (+ (* _index (CallFunction|GetOneMeterConst)) (.X (Math|Vector|BreakVector (LocalVariables|GetL_StartPoint)))) (.Y (Math|Vector|BreakVector (LocalVariables|GetL_StartPoint))) (.Z (Math|Vector|BreakVector (LocalVariables|GetL_StartPoint)))) "0, 0, 0" "1,1,1"))
    (Class|InstancedStaticMeshComponent|AddInstanceWorldSpace (Variables|Default|GetInstancedBlockWalls) (Math|Transform|MakeTransform (+ (Math|Vector|MakeVector (+ (* _index (CallFunction|GetOneMeterConst)) (.X (Math|Vector|BreakVector (LocalVariables|GetL_StartPoint)))) (.Y (Math|Vector|BreakVector (LocalVariables|GetL_StartPoint))) (.Z (Math|Vector|BreakVector (LocalVariables|GetL_StartPoint)))) (Math|Vector|MakeVector 0.0 (* (LocalVariables|GetL_BoxSizeY) (CallFunction|GetOneMeterConst)) 0.0)) "0, 0, 0" "1,1,1")))
  ;[1 1 1] After create two walls from Y coordinate, without first index, because first index be created in X walls
  (for _index_2 (range 1 (Variables|Params|GetWidthY))
    (Class|InstancedStaticMeshComponent|AddInstanceWorldSpace (Variables|Default|GetInstancedBlockWalls) (Math|Transform|MakeTransform (Math|Vector|MakeVector (.X (Math|Vector|BreakVector (LocalVariables|GetL_StartPoint))) (+ (* _index_2 (CallFunction|GetOneMeterConst)) (.Y (Math|Vector|BreakVector (LocalVariables|GetL_StartPoint)))) (.Z (Math|Vector|BreakVector (LocalVariables|GetL_StartPoint)))) "0, 0, 0" "1,1,1"))
    (Class|InstancedStaticMeshComponent|AddInstanceWorldSpace (Variables|Default|GetInstancedBlockWalls) (Math|Transform|MakeTransform (+ (Math|Vector|MakeVector (.X (Math|Vector|BreakVector (LocalVariables|GetL_StartPoint))) (+ (* _index_2 (CallFunction|GetOneMeterConst)) (.Y (Math|Vector|BreakVector (LocalVariables|GetL_StartPoint)))) (.Z (Math|Vector|BreakVector (LocalVariables|GetL_StartPoint)))) (Math|Vector|MakeVector (* (LocalVariables|GetL_BoxSizeX) (CallFunction|GetOneMeterConst)) 0.0 0.0)) "0, 0, 0" "1,1,1"))))

(fn GeneratePointsMapList
  (Utilities|Map|Clear (Variables|Status|GetAreaPoints))
  (for _index (range 0 (- (Variables|Params|GetWidthX) 1))
    (LocalVariables|SetL_XIndex _index)
    (for _index_2 (range 0 (- (Variables|Params|GetWidthY) 1))
      ;[1 1 1] Initialize map with all points is empty
      (LocalVariables|SetL_YIndex _index_2)
      (Utilities|Map|Add (Variables|Status|GetAreaPoints) (Utilities|ParseVectortoVector2dInt (ConstructArena|GetPositionbyIndex (LocalVariables|GetL_XIndex) (LocalVariables|GetL_YIndex))) true))))

(fn SetPointStatusinArea
  (params (Point :type Vector) (SetEmpty :type Boolean))
  (bind _output_get (LocalVariables|SetL_Vector2dInt (Utilities|ParseVectortoVector2dInt Point)))
  (if (Utilities|Map|Contains (Variables|Status|GetAreaPoints) _output_get)
    (Utilities|Map|Add (Variables|Status|GetAreaPoints) (LocalVariables|GetL_Vector2dInt) SetEmpty)
    (return)))

(fn GetEmptyPointonArea
  (bind _areawithignore (ArenaStatus|ConstructIgnorePointwithArea))
  (bind (_emptyfound _emptypoint) (ArenaStatus|FindRandomEmptyPoint _areawithignore))
  (return _emptyfound _emptypoint))

(fn ConstructIgnorePointwithArea
  ;[1 1 1] Set ignor points with fake IsNotEmpty
  (LocalVariables|SetL_Area (Variables|Status|GetAreaPoints))
  (bind _points (Class|BPIPlayerController|GetPointstoIgnore(Message) (Game|GetPlayerController 0)))
  (for _array_element _points
    (Utilities|Map|Add (LocalVariables|GetL_Area) (Utilities|ParseVectortoVector2dInt _array_element) false))
  (return (LocalVariables|GetL_Area)))

(fn FindRandomEmptyPoint
  (params (FindList :type Map%20of%20S%20Vector%202d%20Int%20Structures%20to%20Booleans))
  (bind _l_emptypoints (LocalVariables|GetL_EmptyPoints))
  (bind _keys (Utilities|Map|Keys FindList))
  (for _array_element _keys
    (if (.Value (Utilities|Map|Find FindList _array_element))
      (Utilities|Array|AddUnique (LocalVariables|GetL_EmptyPoints) _array_element)))
  (return (> (Utilities|Array|Length _l_emptypoints) 0) (Utilities|ParseVector2dInttoVector (Utilities|Array|Get(acopy) _l_emptypoints (Math|Random|RandomIntegerinRange 0 (Utilities|Array|LastIndex _l_emptypoints))))))

(fn ResizeGrid
  (params (NewX :type Integer) (NewY :type Integer))
  (Variables|Params|SetWidthX NewX)
  (Variables|Params|SetWidthY NewY)
  (ConstructArena|ConstructFloor)
  (ConstructArena|ConstructBlockWalls)
  (ConstructArena|SetFloortoEqualCenterCoordinate)
  (ConstructArena|GeneratePointsMapList))