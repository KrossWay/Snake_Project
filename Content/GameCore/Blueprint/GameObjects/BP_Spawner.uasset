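; BP_Spawner is an actor that populates a generated level with game objects at empty points.
; GeneratedGameObjects requests a given count of every class in its ActorsToSpwan list, stopping early for a class once no empty point is found.
; Each spawn asks LevelGenerator for an empty point on the area.
; Its event graph is empty, so spawning runs only when these functions are called.
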(event EventBeginPlay)

(event Collision|EventActorBeginOverlap
  (params (OtherActor :type Actor%20Object%20Reference)))

(event EventTick
  (params (DeltaSeconds :type Float%20%28single-precision%29)))

(fn ConstructionScript)

(fn SpawnActoronArea
  (params (ActorToSpawn :type Actor%20Class%20Reference))
  (bind (_emptyfound _point) (Default|GetEmptyPointonArea (Variables|Default|GetLevelGenerator)))
  (if _emptyfound
    (Game|SpawnActorfromClass ActorToSpawn (Math|Transform|MakeTransform _point "0, 0, 0" "1,1,1") "Undefined" 0 0)
    (return true)
    (else
      (return false))))

(fn TrySpawnActorsCount
  (params (ActorToSpawn :type Actor%20Class%20Reference) (Count :type Integer))
  (if (> Count 0)
    (Utilities|FlowControl|ForLoopwithBreak 1 Count :!label _label
      (:LoopBody
        (bind _success (System|SpawnActoronArea ActorToSpawn))
        (if (not _success)
          (goto _label Break)))
      (:Completed
        (return)))
    (else
      (return))))

(fn GeneratedGameObjects
  (params (CountObjects :type Integer))
  (for _array_element (Variables|Default|GetActorsToSpwan)
    (System|TrySpawnActorsCount _array_element CountObjects))
  (return))