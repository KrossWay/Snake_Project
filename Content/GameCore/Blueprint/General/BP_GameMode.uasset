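; Game mode that runs a grid-based score game, from start through score updates to game over.
; On BeginPlay it caps FPS at 60 and spawns a level generator sized to the play area, plus a spawner that references it.
; Starting resets the score and spawns objects; destroyed objects trigger respawn attempts, and cell status and resize requests go to the generator.
; Score changes update the HUD; reaching the win score or player death ends the game through the player controller.
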(event EventBeginPlay
  (System|SetMaxFps)
  (System|SpawnGameClass))

(event EventSetStatusCellonFloor
  (params (Point :type Vector :default "0, 0, 0") (IsEmpty :type Boolean))
  (bind _levelgenerator (Variables|Objects|GetLevelGenerator))
  (Utilities|IsValid _levelgenerator
    (:Is%20Valid
      (Default|SetPointStatusinArea _levelgenerator Point IsEmpty))))

(event EventAddScore
  (params (Score :type Integer))
  (Score|ChangeScore Score))

(event EventGameObjectDestroyed
  (params (ClassActorDestroyed :type Actor%20Class%20Reference))
  (Default|TrySpawnActorsCount (Variables|Objects|GetSpawner) ClassActorDestroyed 1))

(event EventBegintheGame
  (System|GameStart))

(event EventPlayerIsDead
  (System|GameFinished))

(event EventResizeLevelGrid
  (params (XGrid :type Integer) (YGrid :type Integer))
  (System|SetNewSizeGrid XGrid YGrid))

(fn ConstructionScript)

(fn SpawnGameClass
  (bind _returnvalue (Game|SpawnActorfromClass "/Game/GameCore/Blueprint/GameObjects/BP_LevelGenerator.BP_LevelGenerator_C" (Math|Transform|MakeTransform "0, 0,-50.000000" "0, 0, 0" "1,1,1") "Undefined" 0 (Variables|GameInfo|GetPlayAreaSizeX) (Variables|GameInfo|GetPlayAreaSizeY) 0))
  (bind _output_get (Variables|Objects|SetLevelGenerator _returnvalue))
  (bind _returnvalue_2 (Game|SpawnActorfromClass "/Game/GameCore/Blueprint/GameObjects/BP_Spawner.BP_Spawner_C" (Math|Transform|MakeTransform "0, 0, 0" "0, 0, 0" "1,1,1") "Undefined" 0 _output_get 0))
  (Variables|Objects|SetSpawner _returnvalue_2)
  (return))

(fn ChangeScore
  (params (Score :type Integer))
  (bind _output_get (Variables|GameInfo|SetCurrentScore (+ Score (Variables|GameInfo|GetCurrentScore))))
  (Class|BPIHUD|ScoreChanged(Message) (HUD|GetHUD (Game|GetPlayerController 0)) _output_get)
  (System|CheckWinScore)
  (return))

(fn GameStart
  (if (not (Variables|GameInfo|GetGameStarted))
    (Variables|GameInfo|SetGameStarted true)
    (Score|ClearScore)
    (Default|GeneratedGameObjects (Variables|Objects|GetSpawner) (Variables|GameInfo|GetAmountToSpawnObjects))
    (Class|BPIPlayerController|GameStarted(Message) (Game|GetPlayerController 0))
    (return)))

(fn ClearScore
  (bind _output_get (Variables|GameInfo|SetCurrentScore 0))
  (Score|ChangeScore _output_get)
  (return))

(fn CheckWinScore
  (if (>= (Variables|GameInfo|GetCurrentScore) (Variables|GameInfo|GetScoreToWin))
    (System|GameFinished)))

(fn GameFinished
  (Class|BPIPlayerController|GameOver(Message) (Game|GetPlayerController 0) (Variables|GameInfo|GetCurrentScore))
  (return))

(fn SetMaxFps
  (Development|ExecuteConsoleCommand "t.MaxFPS 60" 0)
  (return))

(fn SetNewSizeGrid
  (params (X :type Integer) (y :type Integer))
  (bind _levelgenerator (Variables|Objects|GetLevelGenerator))
  (Variables|GameInfo|SetPlayAreaSizeX X)
  (Variables|GameInfo|SetPlayAreaSizeY y)
  (Utilities|IsValid _levelgenerator
    (:Is%20Valid
      (Default|ResizeGrid _levelgenerator (Variables|GameInfo|GetPlayAreaSizeX) (Variables|GameInfo|GetPlayAreaSizeY))
      (return))))