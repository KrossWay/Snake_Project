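; Player controller that relays input and game state changes to the controlled pawn and HUD through interface messages.
; Fire and movement inputs go to the pawn, while a quit action exits the game.
; GameStarted and GameOver start or stop the pawn and switch between game-only and cursor-visible UI input, with GameOver also showing the end-game window with the score.
; GetPointsToIgnore returns the points around the pawn.
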(event EventGameOver
  (params (TotalScore :type Integer))
  (CallFunction|SetCursorandInputMode true)
  (Class|BPIControlledPawn|StopGame(Message) (Pawn|GetControlledPawn))
  (Class|BPIHUD|ShowEndGameWindow(Message) (HUD|GetHUD) TotalScore))

(event EventBeginPlay
  (CallFunction|SetCursorandInputMode true))

(event EventGameStarted
  (CallFunction|SetCursorandInputMode false)
  (Class|BPIControlledPawn|BeginMoving(Message) (Pawn|GetControlledPawn)))

(event Input|ActionEvents|InputActionFire
  (params (Key :type Key%20Structure :default "None"))
  ;[1 1 1] Input
  (:Pressed
    (Class|BPIControlledPawn|InputFire(Message) (Pawn|GetControlledPawn))))

(event Input|ActionEvents|InputActionQuitGame
  (params (Key :type Key%20Structure :default "None"))
  ;[1 1 1] Input
  (:Pressed
    (Game|QuitGame 0 "Quit" false)))

(event Input|AxisEvents|InputAxisMoveTop
  (params (AxisValue :type Float%20%28single-precision%29))
  ;[1 1 1] Input
  (if (!= AxisValue 0.0)
    (Class|BPIControlledPawn|InputMoveUp(Message) (Pawn|GetControlledPawn) AxisValue)))

(event Input|AxisEvents|InputAxisMoveRight
  (params (AxisValue :type Float%20%28single-precision%29))
  ;[1 1 1] Input
  (if (!= AxisValue 0.0)
    (Class|BPIControlledPawn|InputMoveRight(Message) (Pawn|GetControlledPawn) AxisValue)))

(fn ConstructionScript)

(fn SetCursorandInputMode
  (params (ShowCursor :type Boolean))
  (bind _output_get (Variables|Default|SetbShowMouseCursor ShowCursor))
  (if _output_get
    (Input|SetInputModeUIOnly self 0 "DoNotLock")
    (else
      (Input|SetInputModeGameOnly self))))

(fn GetPointstoIgnore
  (bind _points (Class|BPIControlledPawn|GetPointsAroundPawn(Message) (Pawn|GetControlledPawn)))
  (return _points))